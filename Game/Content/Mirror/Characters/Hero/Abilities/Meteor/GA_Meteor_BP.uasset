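; Hero gameplay ability for Meteor: the player confirms a target point, then a rock spawns high above it.
; While active it raises the camera boom, shows confirm/cancel text and runs a user-confirmed WaitTargetData task, all cleaned up on end.
; On valid data it commits, and only the authority spawns the rock, passing stun and SetByCaller damage effect specs.
; Non-authority, failed commit and cancelled targeting all cancel the ability.
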(event Ability|EventActivateAbility
  (bind _returnvalue (Class|GameplayAbility|MakeTargetLocationInfofromOwnerActor))
  (bind (_locationtype _literaltransform _sourceactor _sourcecomponent _sourceability _sourcesocketname) (Utilities|Struct|BreakGameplayAbilityTargetingLocationInfo _returnvalue))
  (bind _asmrrhero_character (Utilities|Casting|CastToMRRHeroCharacter (Ability|GetAvatarActorfromActorInfo)))
  (Variables|Default|SetOwningHero _asmrrhero_character)
  (bind _asbp_player_state (Utilities|Casting|CastToBP_PlayerState (Ability|GetOwningActorfromActorInfo)))
  (Class|MRRPlayerState|ShowAbilityConfirmCancelText _asbp_player_state true)
  (Transformation|SetRelativeLocation (Variables|/Script/Mirror.MRRHeroCharacter|GetCameraBoom (Variables|Default|GetOwningHero)) (Math|Vector|MakeVector (.x (Variables|/Script/Mirror.MRRHeroCharacter|GetStartingCameraBoomLocation (Variables|Default|GetOwningHero))) (.y (Variables|/Script/Mirror.MRRHeroCharacter|GetStartingCameraBoomLocation (Variables|Default|GetOwningHero))) (+ (.z (Variables|/Script/Mirror.MRRHeroCharacter|GetStartingCameraBoomLocation (Variables|Default|GetOwningHero))) 1e+02)) false false)
  (bind (_asynctaskproxy _data) (|WaitTargetData :ConfirmationType "UserConfirmed" :Class (Variables|Default|GetTargetActorClass) :MaxRange (Variables|Default|GetRange) :StartLocation (Utilities|Struct|MakeGameplayAbilityTargetingLocationInfo _locationtype (Math|Transform|MakeTransform (+ (* (Transformation|GetActorForwardVector (Variables|Default|GetOwningHero)) 2e+02) (.location _literaltransform)) (.rotation _literaltransform) (.scale _literaltransform)) _sourceactor _sourcecomponent _sourceability _sourcesocketname) :ReticleClass 0)
    (:then
      (Variables|Default|SetTargetingTask _asynctaskproxy))
    (:ValidData
      (bind _returnvalue_2 (Ability|CommitAbility))
      (if _returnvalue_2
        (if (Ability|HasAuthority (Variables|Default|GetOwningHero))
          (bind _returnvalue_3 (Ability|GameplayEffect|AssignTagSetbyCallerMagnitude (Ability|MakeOutgoingGameplayEffectSpec (Variables|Default|GetDamageGameplayEffectClass) (Math|Conversions|ToFloat(Integer) (Ability|GetAbilityLevel))) "(TagName=\"Data.Damage\")" (Variables|Default|GetDamage)))
          (Game|SpawnActorfromClass (Variables|Default|GetRockClass) (Math|Transform|MakeTransform (+ (.Location (Collision|BreakHitResult (Ability|TargetData|GetHitResultfromTargetData _data))) "0, 0,3000.000000") "0, 0, 0" "1,1,1") "AlwaysSpawn" (Variables|Default|GetOwningHero) (Ability|MakeOutgoingGameplayEffectSpec (Variables|Default|GetStunGameplayEffectClass) (Math|Conversions|ToFloat(Integer) (Ability|GetAbilityLevel))) 0.0 _returnvalue_3 (Variables|Default|GetOwningHero))
          (Ability|EndAbility)
          (else
            (Ability|CancelAbility :!label _label)))
        (else
          (goto _label))))
    (:Cancelled
      (goto _label))))

(event Ability|EventOnEndAbility
  (params (bWasCancelled :type Boolean))
  (bind _owninghero (Variables|Default|GetOwningHero))
  (Transformation|SetRelativeLocation (Variables|/Script/Mirror.MRRHeroCharacter|GetCameraBoom _owninghero) (Variables|/Script/Mirror.MRRHeroCharacter|GetStartingCameraBoomLocation _owninghero) false false)
  (bind _asmrrplayer_state (Utilities|Casting|CastToMRRPlayerState (Ability|GetOwningActorfromActorInfo)))
  (Class|MRRPlayerState|ShowAbilityConfirmCancelText _asmrrplayer_state false)
  (bind _targetingtask (Variables|Default|GetTargetingTask)
    (:then
      (GameplayTasks|EndTask _targetingtask))
    (:else)))