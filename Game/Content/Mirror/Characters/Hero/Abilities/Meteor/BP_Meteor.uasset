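; BP_Meteor is the hero Meteor ability's actor, which damages and stuns characters it hits.
; The first begin overlap on its collision sphere passes a DoOnce gate, and only the authority then processes the hit.
; It gathers every MRRCharacterBase inside the sphere and applies damage and stun gameplay effect specs to each living one with a valid ability system component.
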(event OnComponentBeginOverlap(SphereCollision)
  (params (OverlappedComponent :type Primitive%20Component%20Object%20Reference) (OtherActor :type Actor%20Object%20Reference) (OtherComp :type Primitive%20Component%20Object%20Reference) (OtherBodyIndex :type Integer) (bFromSweep :type Boolean) (SweepResult :type Hit%20Result%20Structure%20%28by%20ref%29))
  (Utilities|FlowControl|DoOnce false
    (:Completed
      (Networking|SwitchHasAuthority
        (:Authority
          (for _array_element (Collision|GetOverlappingActors (Variables|Default|GetSphereCollision) "/Script/Mirror.MRRCharacterBase" :!class /Script/Engine.PrimitiveComponent)
            (bind _asmrrcharacter_base (Utilities|Casting|CastToMRRCharacterBase _array_element))
            (if (and (Class|MRRCharacterBase|IsAlive _asmrrcharacter_base) (Utilities|IsValid (Ability|GetAbilitySystemComponent _asmrrcharacter_base)))
              (GameplayEffects|ApplyGameplayEffectSpecToSelf (Ability|GetAbilitySystemComponent _asmrrcharacter_base) (Variables|Default|GetDamageEffectSpecHandle))
              (GameplayEffects|ApplyGameplayEffectSpecToSelf (Ability|GetAbilitySystemComponent _asmrrcharacter_base) (Variables|Default|GetStunEffectSpecHandle)))))))))

(fn ConstructionScript)