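; Storm area actor for a Hero ability that damages living characters inside its sphere, then destroys itself.
; On spawn it activates the Storm effect, deactivates it after Duration, and destroys itself after a short delay, during which damage continues.
; A looping timer makes the server apply a GAS damage effect via SetByCaller to overlapping characters.
; Each target's own ASC creates the spec, with no instigator or team filtering.
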(event Custom|DamageTick
  (Networking|SwitchHasAuthority
    (:Authority
      (for _array_element (Collision|GetOverlappingActors (Variables|Default|GetSphereCollision) 0 :!class /Script/Engine.PrimitiveComponent)
        (bind _asmrrcharacter_base (Utilities|Casting|CastToMRRCharacterBase _array_element))
        (if (and (Class|MRRCharacterBase|IsAlive _asmrrcharacter_base) (Utilities|IsValid (Ability|GetAbilitySystemComponent _asmrrcharacter_base)))
          (bind _returnvalue (Ability|GameplayEffect|AssignTagSetbyCallerMagnitude (GameplayEffects|MakeOutgoingSpec (Ability|GetAbilitySystemComponent _asmrrcharacter_base) (Variables|Default|GetDamageGameplayEffectClass) 1.0 (GameplayEffects|MakeEffectContext (Ability|GetAbilitySystemComponent _asmrrcharacter_base))) "(TagName=\"Data.Damage\")" (Variables|Default|GetDamage)))
          (GameplayEffects|ApplyGameplayEffectSpecToSelf (Ability|GetAbilitySystemComponent _asmrrcharacter_base) _returnvalue))))))

(event EventBeginPlay
  (Components|Activation|Activate (Variables|Default|GetStorm) false)
  (Utilities|Time|SetTimerbyEvent (delegate Custom|DamageTick) 0.1 true)
  (Utilities|FlowControl|Delay (Variables|Default|GetDuration))
  (Components|Activation|Deactivate (Variables|Default|GetStorm))
  (Utilities|FlowControl|Delay 3.0)
  (Actor|DestroyActor))

(fn ConstructionScript)