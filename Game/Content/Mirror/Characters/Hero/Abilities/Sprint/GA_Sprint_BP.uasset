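; Hero sprint Gameplay Ability that lasts while input is held and its cost can be paid.
; Activation applies the sprint effect and cue, then starts sprinting on the MRR movement component.
; A short delay loop, net-synced with OnlyServerWait, commits cost only while the hero is grounded and accelerating.
; Input release or a failed cost commit ends the ability, which removes the effect and stops sprinting.
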(event Ability|EventActivateAbility
  (bind _returnvalue (Ability|GetActorInfo))
  (bind _movementcomponent (Utilities|Struct|BreakGameplayAbilityActorInfo _returnvalue))
  (Variables|Default|SetEndSprint false)
  (bind _returnvalue_2 (Ability|ApplyGameplayEffectToOwner "/Game/Mirror/Characters/Shared/GameplayEffectTemplates/GE_StandardSprint.GE_StandardSprint_C" (Ability|GetAbilityLevel)))
  (Variables|Default|SetGESprint _returnvalue_2)
  (GameplayCue|AddGameplayCue :GameplayCueTag "(TagName=\"GameplayCue.Hero.Sprint\")")
  (bind _asmrrcharacter_movement_component (Utilities|Casting|CastToMRRCharacterMovementComponent _movementcomponent))
  (Class|MRRCharacterMovementComponent|StartSprinting _asmrrcharacter_movement_component)
  (Ability|Tasks|WaitInputRelease true
    (:then
      (Ability|Tasks|WaitDelay 0.05 :!label _label
        (:OnFinish
          (Ability|Tasks|WaitNetSync "OnlyServerWait"
            (:OnSync
              (bind _ascharacter_movement_component (Utilities|Casting|CastToCharacterMovementComponent _movementcomponent))
              (if (and (not (AI|Components|NavMovement|IsFalling _ascharacter_movement_component)) (> (Math|Vector|VectorLength (Pawn|Components|CharacterMovement|GetCurrentAcceleration _ascharacter_movement_component)) 0.0))
                (bind _returnvalue_3 (Ability|CommitAbilityCost false))
                (if _returnvalue_3
                  (if (not (Variables|Default|GetEndSprint)) :!label _label_2
                    (goto _label))
                  (else
                    (Variables|Default|SetEndSprint true :!label _label_3)
                    (Ability|EndAbility)))
                (else
                  (goto _label_2))))))))
    (:OnRelease
      (goto _label_3))))

(event Ability|EventOnEndAbility
  (params (bWasCancelled :type Boolean))
  (Ability|RemoveGameplayEffectFromOwnerWithHandle (Variables|Default|GetGESprint))
  (bind _asmrrcharacter_movement_component (Utilities|Casting|CastToMRRCharacterMovementComponent (.MovementComponent (Utilities|Struct|BreakGameplayAbilityActorInfo (Ability|GetActorInfo)))))
  (Class|MRRCharacterMovementComponent|StopSprinting _asmrrcharacter_movement_component))