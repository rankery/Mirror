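; Projectile for the hero's Fireball ability that delivers a GAS damage effect and explodes on hitting objects or reaching max range.
; Lifespan and explosion delay derive from range divided by initial speed.
; The first overlap is processed once; on authority, a character hit re-traces for an accurate HitResult, adds it to the effect context, applies the damage spec and destroys the projectile.
; Other hits, and all non-instigator remote hits, spawn an explosion and destroy it.
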(event OnComponentBeginOverlap(Collision)
  (params (OverlappedComponent :type Primitive%20Component%20Object%20Reference) (OtherActor :type Actor%20Object%20Reference) (OtherComp :type Primitive%20Component%20Object%20Reference) (OtherBodyIndex :type Integer) (bFromSweep :type Boolean) (SweepResult :type Hit%20Result%20Structure%20%28by%20ref%29))
  ;[1 1 1] Hero or object
  (Utilities|FlowControl|DoOnce false
    (:Completed
      (if (!= OtherActor (Game|GetInstigator))
        (Networking|SwitchHasAuthority
          (:Authority
            (bind _asmrrcharacter_base (Utilities|Casting|CastToMRRCharacterBase OtherActor)
              (:then
                ;[1 1 1] Hit hero
                (if (Utilities|IsValid (Ability|GetAbilitySystemComponent _asmrrcharacter_base))
                  (bind _outhits (Class|KismetSystemLibrary|LineTraceMultiforObjects (Transformation|GetActorLocation) (Transformation|GetActorLocation _asmrrcharacter_base) (Utilities|Array|MakeArray "ObjectTypeQuery3") false 0 "ForOneFrame" true "(R=1.000000,G=0.000000,B=0.000000,A=1.000000)" "(R=0.000000,G=1.000000,B=0.000000,A=1.000000)" 2.0))
                  (bind _array_element (Utilities|Array|ForEachLoopwithBreak _outhits :!label _label)
                    (:LoopBody
                      (if (== _asmrrcharacter_base (.HitActor (Collision|BreakHitResult _array_element)))
                        (Variables|Default|SetFinalHit _array_element)
                        (goto _label Break)))
                    (:Completed
                      (bind _returnvalue (Class|AbilitySystemBlueprintLibrary|GetEffectContext (Variables|Default|GetDamageEffectSpecHandle)))
                      (Class|AbilitySystemBlueprintLibrary|EffectContextAddHitResult _returnvalue (Variables|Default|GetFinalHit) false)
                      (GameplayEffects|ApplyGameplayEffectSpecToSelf (Ability|GetAbilitySystemComponent _asmrrcharacter_base) (Variables|Default|GetDamageEffectSpecHandle))
                      (Actor|DestroyActor)))))
              (:CastFailed
                ;[1 1 1] Hit object
                (bind _returnvalue_2 (Class|AbilitySystemBlueprintLibrary|GetEffectContext (Variables|Default|GetDamageEffectSpecHandle) :!label _label_2))
                (Class|AbilitySystemBlueprintLibrary|EffectContextAddHitResult _returnvalue_2 SweepResult false)
                (Effects|SpawnEmitteratLocation "/Game/FXVarietyPack/Particles/P_ky_explosion.P_ky_explosion" (.Location (Collision|BreakHitResult SweepResult)))
                (Actor|DestroyActor))))
          (:Remote
            (goto _label_2)))))))

(event EventBeginPlay
  (bind _projectilemovement (Variables|Default|GetProjectileMovement))
  (bind _range (Variables|Default|GetRange))
  (bind _initialspeed (Variables|/Script/Engine.ProjectileMovementComponent|GetInitialSpeed _projectilemovement))
  (bind _returnvalue (/ _range _initialspeed))
  (Actor|SetLifeSpan _returnvalue)
  (Utilities|FlowControl|Delay _returnvalue)
  (Effects|SpawnEmitteratLocation "/Game/FXVarietyPack/Particles/P_ky_explosion.P_ky_explosion" (Transformation|GetActorLocation)))

(fn ConstructionScript)