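; BP_HealthManaStaminaVolume is a volume that applies a health, mana and stamina gameplay effect to characters inside it.
; A looping one-second timer started at BeginPlay scans the Box's overlapping actors on the server only.
; Each living MRRCharacterBase with a valid Ability System Component gets GE_HealthManaStaminaVolume applied to itself.
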(event Custom|DamageTick
  (Networking|SwitchHasAuthority
    (:Authority
      (for _array_element (Collision|GetOverlappingActors (Variables|Default|GetBox) 0 :!class /Script/Engine.PrimitiveComponent)
        (bind _asmrrcharacter_base (Utilities|Casting|CastToMRRCharacterBase _array_element))
        (if (and (Class|MRRCharacterBase|IsAlive _asmrrcharacter_base) (Utilities|IsValid (Ability|GetAbilitySystemComponent _asmrrcharacter_base)))
          (GameplayEffects|ApplyGameplayEffectToSelf (Ability|GetAbilitySystemComponent _asmrrcharacter_base) "/Game/Mirror/Blueprints/GE_HealthManaStaminaVolume.GE_HealthManaStaminaVolume_C" 1.0 (GameplayEffects|MakeEffectContext (Ability|GetAbilitySystemComponent _asmrrcharacter_base))))))))

(event EventBeginPlay
  (Utilities|Time|SetTimerbyEvent (delegate Custom|DamageTick) 1.0 true))

(fn ConstructionScript)